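; AI controller for evolved human enemies that runs behavior trees from an evolving population and reports their fitness.
; On possess it finds the evolution control actor by tag and takes a population member, retrying when the population becomes ready, or reuses its existing registration.
; It runs that tree, binds a fitness updater component to the member ID, and seeds initial fitness values.
; On unpossess it releases the registration.
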(event Custom|OnTrialPopulationReady
  ;[1 1 1] Find the correct EvolutionControlActor
  (bind _outactors (Class|EvolutionControlActor|GetEvolutionControlActorsbyTag (Variables|Default|GetEvolution%20Control%20Actor%20Tag)))
  (if (Utilities|Array|IsValidIndex _outactors)
    ;[1 1 1] If we already have a behavior tree and ID registration from the population, just run that one!
    (if (== (.id (Utilities|Struct|BreakPopulationReg (Variables|Default|GetPopulationReg))) -1)
      ;[1 1 1] Get a new behavior tree registration (tree and ID) from the population, or otherwise register for an event to wait for the population to be ready and try again.
      (bind (_outregistration _returnvalue) (Class|EvolutionControlActor|TryRetrieveNextPopMember (Utilities|Array|Get(acopy) _outactors) (delegate Custom|OnTrialPopulationReady)))
      (bind _output_get (Variables|Default|SetPopulationReg _outregistration))
      (if _returnvalue
        (CallFunction|RunTreeandRegisterFitness (Utilities|Array|Get(acopy) _outactors) _output_get)
        (CallFunction|SetUpInitialFitnesses (Utilities|Array|Get(acopy) _outactors) (.id (Utilities|Struct|BreakPopulationReg _output_get))))
      (else
        (CallFunction|RunTreeandRegisterFitness (Utilities|Array|Get(acopy) _outactors) (Variables|Default|GetPopulationReg))
        (CallFunction|SetUpInitialFitnesses (Utilities|Array|Get(acopy) _outactors) (.id (Utilities|Struct|BreakPopulationReg (Variables|Default|GetPopulationReg))))))
    (else
      (Development|PrintString "No evolution control actor in scene!" false))))

(event EventBeginPlay)

(event EventTick
  (params (DeltaSeconds :type Float%20%28single-precision%29)))

(event EventPossess
  (params (PossessedPawn :type Pawn%20Object%20Reference))
  ;[1 1 1] Find the correct EvolutionControlActor
  (bind _outactors (Class|EvolutionControlActor|GetEvolutionControlActorsbyTag (Variables|Default|GetEvolution%20Control%20Actor%20Tag)))
  (if (Utilities|Array|IsValidIndex _outactors)
    ;[1 1 1] If we already have a behavior tree and ID registration from the population, just run that one!
    (if (== (.id (Utilities|Struct|BreakPopulationReg (Variables|Default|GetPopulationReg))) -1)
      ;[1 1 1] Get a new behavior tree registration (tree and ID) from the population, or otherwise register for an event to wait for the population to be ready and try again.
      (bind (_outregistration _returnvalue) (Class|EvolutionControlActor|TryRetrieveNextPopMember (Utilities|Array|Get(acopy) _outactors) (delegate Custom|OnTrialPopulationReady)))
      (bind _output_get (Variables|Default|SetPopulationReg _outregistration))
      (if _returnvalue
        (CallFunction|RunTreeandRegisterFitness (Utilities|Array|Get(acopy) _outactors) _output_get)
        (CallFunction|SetUpInitialFitnesses (Utilities|Array|Get(acopy) _outactors) (.id (Utilities|Struct|BreakPopulationReg _output_get))))
      (else
        (CallFunction|RunTreeandRegisterFitness (Utilities|Array|Get(acopy) _outactors) (Variables|Default|GetPopulationReg))
        (CallFunction|SetUpInitialFitnesses (Utilities|Array|Get(acopy) _outactors) (.id (Utilities|Struct|BreakPopulationReg (Variables|Default|GetPopulationReg))))))
    (else
      (Development|PrintString "No evolution control actor in scene!" false))))

(event EventUnPossess
  (params (UnpossessedPawn :type Pawn%20Object%20Reference))
  ;[1 1 1] Find the correct EvolutionControlActor
  (bind _outactors (Class|EvolutionControlActor|GetEvolutionControlActorsbyTag (Variables|Default|GetEvolution%20Control%20Actor%20Tag)))
  (if (Utilities|Array|IsValidIndex _outactors)
    ;[1 1 1] If we have a behavior tree and ID registration from the population, unregister it!
    (if (not (== (.id (Utilities|Struct|BreakPopulationReg (Variables|Default|GetPopulationReg))) -1))
      (bind _returnvalue (Class|EvolutionControlActor|GetPopulationManager (Utilities|Array|Get(acopy) _outactors)))
      (Class|PopulationManager|ReleaseRegistration _returnvalue (.id (Utilities|Struct|BreakPopulationReg (Variables|Default|GetPopulationReg))))
      (Variables|Default|SetPopulationReg (Utilities|Struct|MakePopulationReg -1)))
    (else
      (Development|PrintString "No evolution control actor in scene!" false))))

(fn ConstructionScript)

(fn RunTreeandRegisterFitness
  (params (EvolutionControlActor :type Evolution%20Control%20Actor%20Object%20Reference) (BehaviorTreeRegistration :type Population%20Reg%20Structure))
  (bind (_id _bt) (Utilities|Struct|BreakPopulationReg BehaviorTreeRegistration))
  (Variables|Default|SetPopulationReg BehaviorTreeRegistration)
  (bind _returnvalue (AI|RunBehaviorTree _bt))
  (if _returnvalue
    (CallFunction|MakeandRegisterFitnessUpdater _id EvolutionControlActor)
    (else
      (Development|PrintString "Failed to run behavior tree" false))))

(fn SetUpInitialFitnesses
  (params (EvolutionControlActor :type Evolution%20Control%20Actor%20Object%20Reference) (PopulationMemberID :type Integer))
  ;[1 1 1] Set starting fitness values for Alive and HasNeverMoved to 1
  (CallFunction|SendFitnessUpdate "Alive" 1.0 false)
  (CallFunction|SendFitnessUpdate "HasNeverMoved" 1.0 false))

(fn MakeandRegisterFitnessUpdater
  (params (BehaviorTreeRegistration :type Integer) (EvolutionControlActor :type Evolution%20Control%20Actor%20Object%20Reference))
  (bind _returnvalue (Actor|GetComponentbyClass "/Script/EvolvingBehavior.SingleIDFitnessUpdater"))
  ;[1 1 1] If we have a fitness updater component, set our new population member ID on it and register it with the tracker.
  (Utilities|IsValid _returnvalue
    (:Is%20Valid
      (Class|SingleIDFitnessUpdater|SetID _returnvalue BehaviorTreeRegistration)
      (Class|EvolutionControlActor|RegisterFitnessUpdater EvolutionControlActor _returnvalue))
    (:Is%20Not%20Valid
      ;[1 1 1] If we don't have a fitness updater component, make one and register it.
      (bind _returnvalue_2 (AddComponent|AddSingleIDFitnessUpdater))
      (Class|SingleIDFitnessUpdater|SetID _returnvalue_2 BehaviorTreeRegistration)
      (Class|EvolutionControlActor|RegisterFitnessUpdater EvolutionControlActor _returnvalue_2))))

(fn SendFitnessUpdate
  (params (FitnessKey :type String) (Value :type Float%20%28single-precision%29) (IsDelta :type Boolean))
  (if (> (.id (Utilities|Struct|BreakPopulationReg (Variables|Default|GetPopulationReg))) -1)
    (Class|SingleIDFitnessUpdater|BroadcastFitnessUpdate (Actor|GetComponentbyClass "/Script/EvolvingBehavior.SingleIDFitnessUpdater") FitnessKey Value IsDelta)))
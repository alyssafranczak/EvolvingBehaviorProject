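; AI controller for zombies whose behavior trees come from an evolved population managed by an EvolutionControlActor found by tag.
; On possess, it reuses its registered tree or retrieves the next population member, retrying via callback when the population is ready.
; After starting the tree it registers a SingleIDFitnessUpdater component with the control actor.
; It then broadcasts starting fitness values, including genome size terms that discourage too-large or too-small trees.
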(event Custom|OnTrialPopulationReady
  (bind _populationreg (Variables|Default|GetPopulationReg))
  (bind _id (Utilities|Struct|BreakPopulationReg _populationreg))
  ;[1 1 1] Find the correct EvolutionControlActor
  (bind _outactors (Class|EvolutionControlActor|GetEvolutionControlActorsbyTag (Variables|Default|GetEvolutionControlActorTag)))
  (if (Utilities|Array|IsValidIndex _outactors)
    ;[1 1 1] If we already have a behavior tree and ID registration from the population, just run that one!
    (if (== _id -1)
      ;[1 1 1] Get a new behavior tree registration (tree and ID) from the population, or otherwise register for an event to wait for the population to be ready and try again.
      (bind (_outregistration _returnvalue) (Class|EvolutionControlActor|TryRetrieveNextPopMember (Utilities|Array|Get(acopy) _outactors) (delegate Custom|OnTrialPopulationReady)))
      (if _returnvalue
        (CallFunction|RunTreeandRegisterFitness (Utilities|Array|Get(acopy) _outactors) _outregistration)
        (CallFunction|SetUpInitialFitnesses (Utilities|Array|Get(acopy) _outactors) (.id (Utilities|Struct|BreakPopulationReg _outregistration))))
      (else
        (CallFunction|RunTreeandRegisterFitness (Utilities|Array|Get(acopy) _outactors) _populationreg)
        (CallFunction|SetUpInitialFitnesses (Utilities|Array|Get(acopy) _outactors) _id)))
    (else
      (Development|PrintString "No evolution control actor in scene!" false))))

(event EventTick
  (params (DeltaSeconds :type Float%20%28single-precision%29))
  (|CallParentFunction DeltaSeconds) ; This node is disabled and will not be called.\nDrag off pins to build functionality.
)

(event EventPossess
  (params (PossessedPawn :type Pawn%20Object%20Reference))
  (bind _populationreg (Variables|Default|GetPopulationReg))
  (bind _id (Utilities|Struct|BreakPopulationReg _populationreg))
  ;[1 1 1] Find the correct EvolutionControlActor
  (bind _outactors (Class|EvolutionControlActor|GetEvolutionControlActorsbyTag (Variables|Default|GetEvolutionControlActorTag)))
  (if (Utilities|Array|IsValidIndex _outactors)
    ;[1 1 1] If we already have a behavior tree and ID registration from the population, just run that one!
    (if (== _id -1)
      ;[1 1 1] Get a new behavior tree registration (tree and ID) from the population, or otherwise register for an event to wait for the population to be ready and try again.
      (bind (_outregistration _returnvalue) (Class|EvolutionControlActor|TryRetrieveNextPopMember (Utilities|Array|Get(acopy) _outactors) (delegate Custom|OnTrialPopulationReady)))
      (if _returnvalue
        (CallFunction|RunTreeandRegisterFitness (Utilities|Array|Get(acopy) _outactors) _outregistration)
        (CallFunction|SetUpInitialFitnesses (Utilities|Array|Get(acopy) _outactors) (.id (Utilities|Struct|BreakPopulationReg _outregistration))))
      (else
        (CallFunction|RunTreeandRegisterFitness (Utilities|Array|Get(acopy) _outactors) _populationreg)
        (CallFunction|SetUpInitialFitnesses (Utilities|Array|Get(acopy) _outactors) _id)))
    (else
      (Development|PrintString "No evolution control actor in scene!" false))))

(event EventUnPossess
  (params (UnpossessedPawn :type Pawn%20Object%20Reference)))

(fn ConstructionScript
  (|CallParentFunction))

(fn MakeandRegisterFitnessUpdater
  (params (BehaviorTreeRegistration :type Integer) (EvolutionControlActor :type Evolution%20Control%20Actor%20Object%20Reference))
  (bind _returnvalue (Actor|GetComponentbyClass "/Script/EvolvingBehavior.SingleIDFitnessUpdater"))
  ;[1 1 1] If we have a fitness updater component, set our new population member ID on it and register it with the tracker.
  (Utilities|IsValid _returnvalue
    (:Is%20Valid
      (Class|SingleIDFitnessUpdater|SetID _returnvalue BehaviorTreeRegistration)
      (Class|EvolutionControlActor|RegisterFitnessUpdater EvolutionControlActor _returnvalue))
    (:Is%20Not%20Valid
      ;[1 1 1] If we don't have a fitness updater component, make one and register it.
      (bind _returnvalue_2 (AddComponent|AddSingleIDFitnessUpdater))
      (Class|SingleIDFitnessUpdater|SetID _returnvalue_2 BehaviorTreeRegistration)
      (Class|EvolutionControlActor|RegisterFitnessUpdater EvolutionControlActor _returnvalue_2))))

(fn RunTreeandRegisterFitness
  (params (EvolutionControlActor :type Evolution%20Control%20Actor%20Object%20Reference) (BehaviorTreeRegistration :type Population%20Reg%20Structure))
  (bind (_id _bt) (Utilities|Struct|BreakPopulationReg BehaviorTreeRegistration))
  (Variables|Default|SetPopulationReg BehaviorTreeRegistration)
  (bind _returnvalue (AI|RunBehaviorTree _bt))
  (if _returnvalue
    (CallFunction|MakeandRegisterFitnessUpdater _id EvolutionControlActor)
    (else
      (Development|PrintString "Failed to run behavior tree" false))))

(fn SendFitnessUpdate
  (params (FitnessKey :type String) (Value :type Float%20%28single-precision%29) (IsDelta :type Boolean))
  (if (> (.id (Utilities|Struct|BreakPopulationReg (Variables|Default|GetPopulationReg))) -1)
    (Class|SingleIDFitnessUpdater|BroadcastFitnessUpdate (Actor|GetComponentbyClass "/Script/EvolvingBehavior.SingleIDFitnessUpdater") FitnessKey Value IsDelta)))

(fn SetUpInitialFitnesses
  (params (EvolutionControlActor :type Evolution%20Control%20Actor%20Object%20Reference) (PopulationMemberID :type Integer))
  ;[1 1 1] Set starting fitness values for Alive and HasNeverMoved to 1
  (CallFunction|SendFitnessUpdate "Alive" 1.0 false)
  (CallFunction|SendFitnessUpdate "HasNeverMoved" 1.0 false)
  ;[1 1 1] Determine how big our genome/behavior tree is, and set fitness values to encourage it not to be too big or too small.
  (bind _returnvalue (Class|EvolvingBehaviorBlueprintLibrary|GetSizeOfGenome EvolutionControlActor PopulationMemberID))
  (CallFunction|SendFitnessUpdate "ChromosomeSize" (Math|Conversions|ToFloat(Integer) _returnvalue) false)
  (if (>= (- 6 _returnvalue) 0)
    (CallFunction|SendFitnessUpdate "ChromosomeSizeUnderSix" (Math|Conversions|ToFloat(Integer) (- 6 _returnvalue)) false)))